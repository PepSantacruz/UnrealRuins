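; Projectile actor for the Ruin level that damages enemy characters it overlaps.
; On overlapping an EnemyCharacterRuin other than its Instigator, it applies fixed damage credited to the Instigator's controller, shakes the first player's camera and destroys itself.
; The Destroyed event spawns the explosion particle effect at its location, so the effect plays on any destruction, not only on a hit.
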(event EventBeginPlay)

(event Collision|EventActorBeginOverlap
  (params (OtherActor :type Actor%20Object%20Reference))
  (bind _instigator (Variables|Actor|GetInstigator))
  (bind _asenemy_character_ruin (Utilities|Casting|CastToEnemyCharacterRuin OtherActor))
  (if (not (== _asenemy_character_ruin _instigator))
    (Game|Damage|ApplyDamage _asenemy_character_ruin 5e+01 (Pawn|GetController _instigator) self)
    (Class|PlayerCameraManager|PlayCameraShake (Variables|/Script/Engine.PlayerController|GetPlayerCameraManager (Game|GetPlayerController 0)) "/Game/RuinLevel/Blueprints/assets/Camera/BP_CameraShake.BP_CameraShake_C" 1.0 "CameraLocal" "0, 0, 0")
    (Actor|DestroyActor)))

(event EventTick
  (params (DeltaSeconds :type Float%20%28single-precision%29)))

(event EventDestroyed
  (Effects|SpawnEmitteratLocation "/Game/RuinLevel/Blueprints/assets/Effects/ExplosionParticleSystem.ExplosionParticleSystem" (Transformation|GetActorLocation)))

(fn ConstructionScript)