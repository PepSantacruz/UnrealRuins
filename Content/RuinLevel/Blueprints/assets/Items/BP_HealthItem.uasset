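; BP_HealthItem is a pickup that restores health to a GreyCharacter on overlap.
; It only triggers when the character's Health is below its class default, which serves as the maximum.
; It adds HealtUp to Health, clamps the result between zero and that default, then destroys itself, so the item stays in place for characters at full health.
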(event EventBeginPlay)

(event Collision|EventActorBeginOverlap
  (params (OtherActor :type Actor%20Object%20Reference))
  (bind _asgrey_character (Utilities|Casting|CastToGreyCharacter OtherActor))
  (if (< (Variables|/Game/RuinLevel/Blueprints/assets/Character/ThirdPersonGrey/GreyCharacter.GreyCharacter_C|GetHealth _asgrey_character) (.Health (Utilities|GetClassDefaults (Utilities|GetClass _asgrey_character))))
    (Variables|/Game/RuinLevel/Blueprints/assets/Character/ThirdPersonGrey/GreyCharacter.GreyCharacter_C|SetHealth _asgrey_character (Math|Float|Clamp(Float) (+ (Variables|/Game/RuinLevel/Blueprints/assets/Character/ThirdPersonGrey/GreyCharacter.GreyCharacter_C|GetHealth _asgrey_character) (Variables|Default|GetHealtUp)) 0.0 (.Health (Utilities|GetClassDefaults (Utilities|GetClass _asgrey_character)))))
    (Actor|DestroyActor)))

(event EventTick
  (params (DeltaSeconds :type Float%20%28single-precision%29)))

(fn ConstructionScript)